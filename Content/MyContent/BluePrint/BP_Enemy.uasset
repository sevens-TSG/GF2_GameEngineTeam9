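; BP_Enemy is a turret-like enemy that shoots at the player and explodes when hit by a player bullet.
; Each Tick, unless the player pawn equals FlyingPawn, Sphere turns toward the player.
; A Delay in Tick throttles BP_EnemyBullet spawns to about one per second, using Sphere's transform with halved rotation.
; Sphere1 overlap with BP_PlayerBullet spawns an enlarged explosion effect and destroys the enemy.
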(event OnComponentBeginOverlap(Sphere1)
  (params (OverlappedComponent :type Primitive%20Component%20Object%20Reference) (OtherActor :type Actor%20Object%20Reference) (OtherComp :type Primitive%20Component%20Object%20Reference) (OtherBodyIndex :type Integer) (bFromSweep :type Boolean) (SweepResult :type Hit%20Result%20Structure%20%28by%20ref%29))
  (bind _sphere (Variables|Default|GetSphere))
  (bind _returnvalue (Transformation|GetWorldTransform _sphere))
  (Utilities|Casting|CastToBP_PlayerBullet OtherActor)
  (Game|SpawnActorfromClass "/Game/StarterContent/Blueprints/Blueprint_Effect_Explosion.Blueprint_Effect_Explosion_C" (Math|Transform|MakeTransform (.location _returnvalue) (.rotation _returnvalue) (* (.scale _returnvalue) 5.0)) "Undefined" 0 0)
  (Actor|DestroyActor))

(event EventBeginPlay)

(event Collision|EventActorBeginOverlap
  (params (OtherActor :type Actor%20Object%20Reference)))

(event EventTick
  (params (DeltaSeconds :type Float%20%28single-precision%29))
  (bind _returnvalue (Game|Player|GetPlayerPawn 0))
  (bind _sphere (Variables|Default|GetSphere))
  (bind _returnvalue_2 (Transformation|GetWorldTransform _sphere))
  (if (not (== _returnvalue "/Game/FlyingBP/Blueprints/FlyingPawn.FlyingPawn"))
    (Transformation|SetWorldRotation _sphere (Math|Rotator|FindLookatRotation (Transformation|GetActorLocation) (Transformation|GetActorLocation _returnvalue)) false false)
    (Utilities|FlowControl|Delay 1.0)
    (Game|SpawnActorfromClass "/Game/MyContent/BluePrint/BP_EnemyBullet.BP_EnemyBullet_C" (Math|Transform|MakeTransform (.location _returnvalue_2) (* (.rotation _returnvalue_2) 0.5) (.scale _returnvalue_2)) "Undefined" 0 0)))

(fn ConstructionScript)